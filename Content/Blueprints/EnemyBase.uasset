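; EnemyBase is an enemy pawn that walks to one of four end points when play begins.
; On BeginPlay it finds the EnemyController2 actor and copies its SpawnPointNumber into SpawnPointSelected.
; A chain of branches matches that number to the corresponding EndPoint reference and issues AIMoveTo toward that actor with a tight acceptance radius.
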(event EventBeginPlay
  (bind _returnvalue (Actor|GetActorOfClass "/Game/Blueprints/EnemyController2.EnemyController2_C"))
  (bind _asenemy_controller_2 (Utilities|Casting|CastToEnemyController2 _returnvalue))
  (Variables|Default|SetSpawnPointSelected (Variables|/Game/Blueprints/EnemyController2.EnemyController2_C|GetSpawnPointNumber _asenemy_controller_2))
  (if (== (Variables|Default|GetSpawnPointSelected) 1)
    (AI|AIMoveTo self "0, 0, 0" (Utilities|ResolveSoftReference (Variables|Default|GetEndPoint1)) 1.0 false)
    (elif (== (Variables|Default|GetSpawnPointSelected) 2)
      (AI|AIMoveTo self "0, 0, 0" (Utilities|ResolveSoftReference (Variables|Default|GetEndPoint2)) 1.0 false)
      (elif (== (Variables|Default|GetSpawnPointSelected) 3)
        (AI|AIMoveTo self "0, 0, 0" (Utilities|ResolveSoftReference (Variables|Default|GetEndPoint3)) 1.0 false)
        (elif (== (Variables|Default|GetSpawnPointSelected) 4)
          (AI|AIMoveTo self "0, 0, 0" (Utilities|ResolveSoftReference (Variables|Default|GetEndPoint4)) 1.0 false))))))

(fn ConstructionScript)