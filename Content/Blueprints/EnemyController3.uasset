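; Enemy controller that spawns an EnemyBase at one of four random spawn points on BeginPlay, then repeats on a looping 3-second retriggerable delay.
; Each spawn increments EnemyCounter and appends random button codes to ButtonSequence, which is never cleared here, then prints the whole array as A/B/X/Y/L/R.
; IncreaseMaxButtonSequence is never called here; its nested EnemyCounter checks only act at ten or fewer enemies, ending at the highest maximum.
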(event EventBeginPlay
  (Development|PrintString "Enemy Controller Present")
  (Utilities|FlowControl|Sequence
    (:then_0
      (CallFunction|SpawnEnemy :!label _label)
      (Variables|Default|SetEnemyCounter (+ 1 (Variables|Default|GetEnemyCounter)))
      (CallFunction|SelectSequence)
      (Utilities|FlowControl|RetriggerableDelay 3.0 :!label _label_2)
      (goto _label))
    (:then_1
      (goto _label_2))))

(fn ConstructionScript)

(fn SpawnEnemy
  (Variables|Default|SetSpawnPointNumber (Math|Random|RandomIntegerinRange 1 4))
  (if (== (Variables|Default|GetSpawnPointNumber) 1)
    (Development|PrintString "Set Spawn Point 1")
    (Variables|Default|SetSpawnNum (Variables|Default|GetSpawnPoint1))
    (Game|SpawnActorfromClass "/Game/Blueprints/EnemyBase.EnemyBase_C" (Transformation|GetActorTransform (Utilities|ResolveSoftReference (Variables|Default|GetSpawnNum))) "Undefined" 0 0 :!label _label)
    (Development|PrintString "Spawned Enemy")
    (elif (== (Variables|Default|GetSpawnPointNumber) 2)
      (Development|PrintString "Set Spawn Point 2")
      (Variables|Default|SetSpawnNum (Variables|Default|GetSpawnPoint2))
      (goto _label)
      (elif (== (Variables|Default|GetSpawnPointNumber) 3)
        (Development|PrintString "Set Spawn Point 3")
        (Variables|Default|SetSpawnNum (Variables|Default|GetSpawnPoint3))
        (goto _label)
        (elif (== (Variables|Default|GetSpawnPointNumber) 4)
          (Development|PrintString "Set Spawn Point 4")
          (Variables|Default|SetSpawnNum (Variables|Default|GetSpawnPoint4))
          (goto _label))))))

(fn SelectSequence
  (bind _output_get (Variables|Default|SetNumOfButtonsInSequence (Math|Random|RandomIntegerinRange (Variables|Default|GetMinButtonSequence) (Variables|Default|GetMaxButtonSequence))))
  (for _index (range 1 _output_get)
    (bind _output_get_2 (Variables|Default|SetButtonSelection (Math|Random|RandomIntegerinRange 1 6)))
    (Utilities|Array|Add (Variables|Default|GetButtonSequence) _output_get_2))
  (for _array_element (Variables|Default|GetButtonSequence)
    (bind _output_get_3 (Variables|Default|SetArrayValue _array_element))
    (if (== 1 _output_get_3)
      (Development|PrintString "A")
      (elif (== 2 (Variables|Default|GetArrayValue))
        (Development|PrintString "B")
        (elif (== 3 (Variables|Default|GetArrayValue))
          (Development|PrintString "X")
          (elif (== 4 (Variables|Default|GetArrayValue))
            (Development|PrintString "Y")
            (elif (== 5 (Variables|Default|GetArrayValue))
              (Development|PrintString "L")
              (elif (== 6 (Variables|Default|GetArrayValue))
                (Development|PrintString "R")))))))))

(fn IncreaseMaxButtonSequence
  (if (>= 10 (Variables|Default|GetEnemyCounter))
    (Variables|Default|SetMaxButtonSequence 3)
    (if (>= 15 (Variables|Default|GetEnemyCounter))
      (Variables|Default|SetMaxButtonSequence 4)
      (if (>= 20 (Variables|Default|GetEnemyCounter))
        (Variables|Default|SetMaxButtonSequence 5)
        (if (>= 25 (Variables|Default|GetEnemyCounter))
          (Variables|Default|SetMaxButtonSequence 6))))))