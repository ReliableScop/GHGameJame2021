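; Player controller that moves the player character in discrete steps in response to Up and Down input actions.
; On BeginPlay it casts the first player's pawn to BPP_PlayerCharacter and caches it as ControlledPawn.
; Each press offsets that pawn's world transform by MoveAmount, negated for Down, without sweep, so movement ignores collision.
; An unconnected AddMovementInput node remains unused.
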(event EventBeginPlay
  (bind _asbpp_player_character (Utilities|Casting|CastToBPP_PlayerCharacter (Game|Player|GetPlayerPawn 0)))
  (Variables|Default|SetControlledPawn _asbpp_player_character))

(event EventTick
  (params (DeltaSeconds :type Float%20%28single-precision%29)))

(event Input|ActionEvents|InputActionUp
  (params (Key :type Key%20Structure :default "None"))
  (:Pressed
    (Class|Actor|AddActorWorldTransform (Variables|Default|GetControlledPawn) (Math|Transform|MakeTransform (Variables|Default|GetMoveAmount)) false false)))

(event Input|ActionEvents|InputActionDown
  (params (Key :type Key%20Structure :default "None"))
  (:Pressed
    (Class|Actor|AddActorWorldTransform (Variables|Default|GetControlledPawn) (Math|Transform|MakeTransform (* (Variables|Default|GetMoveAmount) (Math|Conversions|ToVector(Float) -1.0))) false false)))

(fn ConstructionScript)