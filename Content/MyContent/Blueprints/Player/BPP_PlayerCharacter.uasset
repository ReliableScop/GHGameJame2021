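; Player character for a lane-based game that occupies one active BPA_Lane at a time.
; BeginPlay gathers all lanes, reorders the array in place by each lane's ActorIndex, then picks ActiveLane through RandomInteger with max zero.
; The MovePlayer event sets the capsule to the active lane's PlayerLocation transform.
; Tick prints lane debug info; CreateSortedArray duplicates the reordering but is never called.
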(event Custom|MovePlayer
  (Transformation|SetWorldTransform (Variables|Collision|GetCapsuleComponent) (Variables|/Game/MyContent/Blueprints/Lanes/BPA_Lane.BPA_Lane_C|GetPlayerLocation (Variables|Default|GetActiveLane)) false false))

(event EventBeginPlay
  (bind _outactors (Actor|GetAllActorsOfClass "/Game/MyContent/Blueprints/Lanes/BPA_Lane.BPA_Lane_C"))
  (bind _output_get (Variables|Default|SetLanes _outactors))
  (for _array_element _output_get
    (Utilities|Array|SetArrayElem _output_get (Variables|/Game/MyContent/Blueprints/Lanes/BPA_Lane.BPA_Lane_C|GetActorIndex _array_element) _array_element))
  (Variables|Default|SetActiveLane (Utilities|Array|Get(acopy) (Variables|Default|GetLanes) (Math|Random|RandomInteger 0))))

(event Collision|EventActorBeginOverlap
  (params (OtherActor :type Actor%20Object%20Reference)))

(event EventTick
  (params (DeltaSeconds :type Float%20%28single-precision%29))
  (bind _lanes (Variables|Default|GetLanes))
  (Development|PrintString (Utilities|GetDisplayName (Variables|Default|GetActiveLane)) true true "(R=0.000000,G=0.660000,B=1.000000,A=1.000000)" DeltaSeconds)
  (Development|PrintString (Utilities|String|Append "There are " (Utilities|String|ToString(Integer) (Utilities|Array|Length _lanes)) " lanes") true true "(R=0.000000,G=0.660000,B=1.000000,A=1.000000)" DeltaSeconds)
  (for _array_element _lanes
    (Development|PrintString (Utilities|GetDisplayName _array_element) true true "(R=0.000000,G=0.660000,B=1.000000,A=1.000000)" DeltaSeconds)))

(fn ConstructionScript)

(fn CreateSortedArray
  (bind _outactors (Actor|GetAllActorsOfClass "/Game/MyContent/Blueprints/Lanes/BPA_Lane.BPA_Lane_C"))
  (for _array_element _outactors
    (Utilities|Array|SetArrayElem _outactors (Variables|/Game/MyContent/Blueprints/Lanes/BPA_Lane.BPA_Lane_C|GetActorIndex _array_element) _array_element)))